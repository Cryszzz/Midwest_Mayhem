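; Player car that steers laterally past branches, deer and gas cans, with all game stats kept on a Global actor.
; Overlaps destroy tagged objects: branches cost health scaled by armor, deer add count and random dollars, cans refill gas.
; Turn input moves along X with Perlin drift, gated by Y-position limits and pause state.
; Tick adds Perlin jitter that grows as health drops, cosine yaw wobble, and highbeam-upgrade headlights.
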(event EventBeginPlay)

(event EventTick
  (params (DeltaSeconds :type Float%20%28single-precision%29))
  (bind _returnvalue (Transformation|GetActorRotation))
  (bind _returnvalue_2 (Utilities|Time|GetTimeSeconds))
  (bind _headlightr (Variables|Default|GetHeadlightR))
  (bind (_roll _pitch _yaw) (Math|Rotator|BreakRotator _returnvalue))
  ;[1 1 1] Car Jitter Animation
  ;;[1 1 1] Positive Feedback
  (bind _returnvalue_3 (Actor|GetActorOfClass "/Game/Gameplay/Global.Global_C"))
  (Transformation|SetActorLocation (+ (Transformation|GetActorLocation) (Math|Vector|MakeVector (* (/ (* (Variables|/Game/Gameplay/Global.Global_C|GetMaxHealth _returnvalue_3) 4.0) (Variables|/Game/Gameplay/Global.Global_C|GetHealth _returnvalue_3)) (Class|KismetMathLibrary|PerlinNoise1D _returnvalue_2)) 0.0 0.0)) false false)
  (Transformation|SetActorRotation (Math|Rotator|MakeRotator _roll _pitch (+ (* (Math|Trig|Cos(Radians) (+ (* _returnvalue_2 1e+01) (* (Math|Trig|GetPI) -0.22))) (/ 1 (Math|Conversions|ToFloat(Integer) (Math|Integer|Max(Integer) 0 1)))) _yaw)))
  ;[1 1 1] Highbeams Upgrade
  (bind _returnvalue_4 (Actor|GetActorOfClass "/Game/Gameplay/Global.Global_C"))
  (if (Variables|/Game/Gameplay/Global.Global_C|GethasHighbeamsUpgrade _returnvalue_4)
    (Rendering|Components|Light|SetLightColor (Variables|Default|GetHeadlightL) "(R=0.101047,G=0.226887,B=0.776042,A=1.000000)" true)
    (Rendering|Components|Light|SetIntensity _headlightr 5e+04)
    (Rendering|Lighting|SetAttenuationRadius _headlightr 1e+04)))

(event Collision|EventActorBeginOverlap
  (params (OtherActor :type Actor%20Object%20Reference))
  ;[1 1 1] Hit Objects
  (bind _returnvalue (Actor|GetActorOfClass "/Game/Gameplay/Global.Global_C"))
  (if (Actor|ActorHasTag OtherActor "Branch")
    (Actor|DestroyActor OtherActor)
    (Variables|/Game/Gameplay/Global.Global_C|SetHealth _returnvalue (+ (Variables|/Game/Gameplay/Global.Global_C|GetHealth _returnvalue) (* (Variables|/Game/Gameplay/Global.Global_C|GetArmorMultiplier _returnvalue) -1.0)))
    (elif (Actor|ActorHasTag OtherActor "Deer")
      (Actor|DestroyActor OtherActor)
      (Variables|/Game/Gameplay/Global.Global_C|SetDeerCount _returnvalue (+ (Variables|/Game/Gameplay/Global.Global_C|GetDeerCount _returnvalue) 1))
      (Variables|/Game/Gameplay/Global.Global_C|SetDeerDollars _returnvalue (+ (Variables|/Game/Gameplay/Global.Global_C|GetDeerDollars _returnvalue) (Math|Random|RandomIntegerinRange 1 5)))
      (elif (Actor|ActorHasTag OtherActor "GasCan")
        (Actor|DestroyActor OtherActor)
        (Variables|/Game/Gameplay/Global.Global_C|SetGas _returnvalue (Math|Float|Min(Float) (Variables|/Game/Gameplay/Global.Global_C|GetMaxGas _returnvalue) (+ (Variables|/Game/Gameplay/Global.Global_C|GetGas _returnvalue) (Variables|/Game/Gameplay/Global.Global_C|GetGasCanAmount _returnvalue))))))))

(event Input|AxisEvents|InputAxisTurn
  (params (AxisValue :type Float%20%28single-precision%29))
  (bind _returnvalue (Transformation|GetActorLocation))
  (bind _y (Math|Vector|BreakVector _returnvalue))
  ;[1 1 1] Lateral Movement on Key Press
  ;;[1 1 1] Boundary Conditions
  (if (<= _y 425.0)
    (if (>= _y -425.0)
      (if (not (Game|IsGamePaused)) :!label _label
        (Transformation|SetActorLocation (+ _returnvalue (Math|Vector|MakeVector (* (+ (* AxisValue 1e+01) (* 7.0 (Class|KismetMathLibrary|PerlinNoise1D (Utilities|Time|GetTimeSeconds)))) -1.0) 0.0 0.0)) false false))
      (elif (> AxisValue 0.0)
        (goto _label)))
    (elif (< AxisValue 0.0)
      (goto _label))))

(fn ConstructionScript)