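; CarBP is a simple car Blueprint that slides sideways in response to player input.
; The Turn input axis offsets the actor's location along world Y by a scaled axis value, without sweep or frame-time scaling.
; An unconnected node chain that would yaw the car around the Z axis never runs, and the construction script and other events are empty.
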(event EventBeginPlay)

(event Collision|EventActorBeginOverlap
  (params (OtherActor :type Actor%20Object%20Reference)))

(event EventTick
  (params (DeltaSeconds :type Float%20%28single-precision%29)))

(event Input|AxisEvents|InputAxisTurn
  (params (AxisValue :type Float%20%28single-precision%29))
  (Transformation|SetActorLocation (+ (Transformation|GetActorLocation) (Math|Vector|MakeVector 0.0 (* AxisValue 5.0) 0.0)) false false))

(fn ConstructionScript)